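; InvisibleWall is a moving kill boundary that ends the game when the player touches it.
; A looping one-second timer started on BeginPlay teleports its root component a fixed step along negative X.
; When an actor tagged Player begins overlapping its Box, it pauses the game, shows the LoseMenu widget and switches to cursor-driven, UI-only input.
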(event OnComponentBeginOverlap(Box)
  (params (OverlappedComponent :type Primitive%20Component%20Object%20Reference) (OtherActor :type Actor%20Object%20Reference) (OtherComp :type Primitive%20Component%20Object%20Reference) (OtherBodyIndex :type Integer) (bFromSweep :type Boolean) (SweepResult :type Hit%20Result%20Structure%20%28by%20ref%29))
  (bind _returnvalue (Game|GetPlayerController 0))
  (if (Actor|ActorHasTag OtherActor "Player")
    (Game|SetGamePaused true)
    (bind _returnvalue_2 (UserInterface|CreateWidget "/Game/FlyGame/MainMenu/Widgets/LoseMenu.LoseMenu_C" _returnvalue))
    (UserInterface|Viewport|AddtoViewport _returnvalue_2 0)
    (Variables|/Script/Engine.PlayerController|SetbShowMouseCursor _returnvalue true)
    (Input|SetInputModeUIOnly _returnvalue 0 "DoNotLock")))

(event Custom|MoveWall
  (Transformation|AddRelativeLocation (Variables|Default|GetDefaultSceneRoot) (Math|Vector|MakeVector -2.5e+03 0.0 0.0) false true))

(event EventBeginPlay
  (Utilities|Time|SetTimerbyEvent (delegate Custom|MoveWall) 1.0 true))

(fn ConstructionScript)