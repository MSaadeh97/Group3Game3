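; PhysicsJet is a player-flown, physics-driven jet with a timed score, missiles and lives.
; Axis inputs apply local thrust and pitch/roll impulses, while Tick adds nose-direction stabilizing force and, at speed, drag along a velocity-aligned HeadingArm.
; Fire spawns bullets with a cooldown, H refills ammo and lives, and obstacle hits cost lives until the lose menu pauses the game.
; Checkpoint reset exists; idle thrust and lift are disconnected.
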(event OnComponentBeginOverlap(JetModel)
  (params (OverlappedComponent :type Primitive%20Component%20Object%20Reference) (OtherActor :type Actor%20Object%20Reference) (OtherComp :type Primitive%20Component%20Object%20Reference) (OtherBodyIndex :type Integer) (bFromSweep :type Boolean) (SweepResult :type Hit%20Result%20Structure%20%28by%20ref%29))
  (bind _audio (Variables|Default|GetAudio))
  (if (Actor|ActorHasTag OtherActor "Obstacles")
    (Actor|DestroyActor OtherActor)
    (Audio|PlaySound2D "/Game/ArtAssets/Audio/SFX/qubodup-BangMid.qubodup-BangMid" 0.5 1.0 0.0 0 0)
    (bind _result (Math|Integer|DecrementInt (Variables|Default|GetLives))
      (:%20%20
        (Effects|SpawnEmitteratLocation "/Game/StarterContent/Particles/P_Steam_Lit.P_Steam_Lit" (Transformation|GetWorldLocation (Variables|Default|GetJetModel)))
        (if (<= _result 0)
          (bind _returnvalue (UserInterface|CreateWidget "/Game/FlyGame/MainMenu/Widgets/LoseMenu.LoseMenu_C"))
          (UserInterface|Viewport|AddtoViewport _returnvalue 0)
          (Game|SetGamePaused true)
          (Audio|Components|Audio|SetSound _audio "/Game/ArtAssets/Audio/lose_music_3_-_1_0.lose_music_3_-_1_0")
          (Audio|Components|Audio|Play _audio 0.0))))))

(event Custom|resetposition
  (bind _jetmodel (Variables|Default|GetJetModel))
  ;[1 1 1] Checkpoint
  (Transformation|SetActorLocation (Components|GetOwner _jetmodel) (Variables|Default|GetCheckpoint) false false)
  (Class|PrimitiveComponent|SetAllPhysicsLinearVelocity _jetmodel "0, 0, 0" false))

(event Custom|Increment%20Score
  (Math|Integer|IncrementInt (Variables|Default|GetScore)))

(event EventBeginPlay
  (Utilities|Time|SetTimerbyEvent (delegate Custom|Increment%20Score) 0.1 true)
  (Audio|Components|Audio|Play (Variables|Default|GetAudio) 0.0))

(event EventTick
  (params (DeltaSeconds :type Float%20%28single-precision%29))
  (bind _jetmodel (Variables|Default|GetJetModel))
  ;[1 1 1] Update Heading Indicator
  (Transformation|SetWorldRotation (Variables|Default|GetHeadingArm) (Math|Conversions|RotationFromXVector (Transformation|GetComponentVelocity (Variables|Default|GetJetModel))) false false) ; Rotates heading indicator to velocity
  (Utilities|FlowControl|Sequence
    (:then_0
      ;[1 1 1] Basic Stabilization
      (Physics|AddForce _jetmodel (Math|Transform|TransformDirection (Transformation|GetActorTransform) (Math|Vector|MakeVector (Variables|Default|GetStabilizingForce) 0.0 0.0)) "None" true) ; Force is direction of aircraft nose
      (if (> (Math|Vector|VectorLength (Transformation|GetComponentVelocity _jetmodel)) 1e+03)
        (Physics|AddForce _jetmodel (* (Math|Vector|GetForwardVector (Variables|Default|GetHeadingArm)) (* (Variables|Default|GetDragForce) -1.0)) "None" true) ; Force is opposite to heading
      ))))

(event Input|ActionEvents|InputActionFire
  (params (Key :type Key%20Structure :default "None"))
  (bind _gun (Variables|Default|GetGun))
  (bind _returnvalue (Transformation|GetWorldTransform _gun))
  (:Pressed
    (Audio|PlaySound2D "/Game/ArtAssets/Audio/SFX/cannon_03.cannon_03" 0.3 1.0 0.0 0 0)
    (if (> (Variables|Default|GetMissles) 0)
      (Utilities|FlowControl|DoOnce false :!label _label
        (:Completed
          (Game|SpawnActorfromClass "/Game/FlyGame/Blueprints/Bullets/BulletTemp.BulletTemp_C" (Math|Transform|MakeTransform (.location _returnvalue) (.rotation _returnvalue) "1,1,1") "Undefined" 0 0)
          (Math|Integer|DecrementInt (Variables|Default|GetMissles)
            (:%20%20
              (Utilities|FlowControl|Delay 0.5)
              (goto _label Reset))))))))

(event Input|AxisEvents|InputAxisMoveUp
  (params (AxisValue :type Float%20%28single-precision%29))
  ;[1 1 1] Pitch Input
  (Class|PrimitiveComponent|AddAngularImpulseinDegrees (Variables|Default|GetJetModel) (Math|Transform|TransformDirection (Transformation|GetActorTransform) (Math|Vector|MakeVector 0.0 (* AxisValue (Variables|Default|GetPitchForceMultiplier)) 0.0)) "None" true))

(event Input|AxisEvents|InputAxisMoveRight
  (params (AxisValue :type Float%20%28single-precision%29))
  ;[1 1 1] Roll Input
  (Class|PrimitiveComponent|AddAngularImpulseinDegrees (Variables|Default|GetJetModel) (Math|Transform|TransformDirection (Transformation|GetActorTransform) (Math|Vector|MakeVector (* (* AxisValue -1.0) (Variables|Default|GetRollForceMultiplier)) 0.0 0.0)) "None" true))

(event Input|AxisEvents|InputAxisThrust
  (params (AxisValue :type Float%20%28single-precision%29))
  ;[1 1 1] Thrust Input
  (Physics|AddForce (Variables|Default|GetJetModel) (Math|Transform|TransformDirection (Transformation|GetActorTransform) (Math|Vector|MakeVector (* AxisValue (Variables|Default|GetThrustForceMultiplier)) 0.0 0.0)) "None" true)
  (Rendering|SetVisibility (Variables|Default|GetThrustFlame) (> AxisValue 0.0) false))

(event Input|KeyboardEvents|H
  (params (Key :type Key%20Structure :default "None"))
  (:Pressed
    (Variables|Default|SetMissles 100)
    (Variables|Default|SetLives 3)))

(fn ConstructionScript)